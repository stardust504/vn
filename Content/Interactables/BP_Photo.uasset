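; BP_Photo is an interactable photo that plays a memory monologue and then opens the way onward.
; On begin play, after a short delay, it gets the HUD from the player character and binds to its printing-finished callback.
; Interacting prints the hardcoded Russian text on the HUD and sets a flag.
; When printing finishes with that flag set, it waits briefly and, only once, sends an open-door message to actors tagged "door1".
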(event `self.ReceiveBeginPlay`
  (`parent.ReceiveBeginPlay`)
  (`KismetSystemLibrary.Delay` 1.0)
  (bind _asbp_my_character (cast `/Game/PlayerSystem/BP_MyCharacter` (`GameplayStatics.GetPlayerCharacter` 0)))
  (bind _output_get (set `self.Character` _asbp_my_character))
  (bind _output_get_2 (set `self.HUD` (`/Game/PlayerSystem/BP_MyCharacter.HUD_Ref` _output_get)))
  (add `/Game/UI/Widgets/WBP_HUD.PrintingFinished` _output_get_2 (`|CreateDelegate` :!event `FinishPrinting`)))

(event `self.Interact`
  (bind _hud (`self.HUD`))
  (`/Engine/EditorBlueprintResources/StandardMacros.IsValid` _hud
    (:`Is Valid`
      (`/Game/UI/Widgets/WBP_HUD.ClearText` _hud)
      (`/Game/UI/Widgets/WBP_HUD.PrintText` _hud "«Это мы с... с кем? Я знаю это лицо. Но не могу вспомнить. Почему я не могу вспомнить?» \n«Моя... подруга? Да. Подруга. Мы смеялись. Было время, когда мы смеялись.» \n«Время идти. Меня ждут. Мой день рождения. Мой идеальный день».")
      (set `self.bInteracted` true))))

(event `FinishPrinting`
  (if (`self.bInteracted`)
    (`/Engine/EditorBlueprintResources/StandardMacros.DoOnce` false
      (:`Completed`
        (`KismetSystemLibrary.Delay` 1.0)
        (bind _outactors (`GameplayStatics.GetAllActorsWithTag` "door1"))
        (for _array_element _outactors
          (message `/Game/Assets/Door/BPI_Door.OpenDoor` _array_element))))))

(fn `GetItemType`
  (returns (Type :type Integer))
  (return 1))

(fn `UserConstructionScript`
  (`parent.UserConstructionScript`))