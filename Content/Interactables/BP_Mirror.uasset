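; BP_Mirror is an interactable broken mirror that gates a shard-collection minigame behind a narrative prompt.
; On BeginPlay it caches the player controller, character and, after a zero-second delay, the character's HUD reference.
; Interact checks for exactly four collected shards: if met, it prints Russian story text and, after a short delay, starts WBP_Minigame_Mirror through the controller; otherwise it prints a hint to find the shards.
; GetItemType returns a fixed type ID.
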(event `self.ReceiveBeginPlay`
  (`parent.ReceiveBeginPlay`)
  (bind _asbp_my_player_controller (cast `/Game/PlayerSystem/BP_MyPlayerController` (`GameplayStatics.GetPlayerController` 0)))
  (set `self.PlayerController` _asbp_my_player_controller)
  (bind _asbp_my_character (cast `/Game/PlayerSystem/BP_MyCharacter` (`GameplayStatics.GetPlayerCharacter` 0)))
  (bind _output_get (set `self.PlayerCharacter` _asbp_my_character))
  (`KismetSystemLibrary.Delay` 0.0)
  (set `self.HUD Ref` (`/Game/PlayerSystem/BP_MyCharacter.HUD_Ref` _output_get)))

(event `/Game/Interactables/BPI_Interact.Interact`
  (if (== (`/Game/PlayerSystem/BP_MyCharacter.CollectedShards` (`self.PlayerCharacter`)) 4)
    (`/Game/UI/Widgets/WBP_HUD.PrintText` (`self.HUD Ref`) "\"Все осколки здесь. Четыре кусочка правды.\" \n\"В каждом — воспоминание. Один ответ — правда. Другой — ложь, которую я сама себе рассказывала.\" \n\"Я должна вспомнить, кто я на самом деле.\"")
    (`KismetSystemLibrary.Delay` 1.0)
    (`/Game/PlayerSystem/BP_MyPlayerController.StartMiniGame` (`self.PlayerController`) "/Game/UI/Widgets/WBP_Minigame_Mirror.WBP_Minigame_Mirror_C")
    (else
      (`/Game/UI/Widgets/WBP_HUD.PrintText` (`self.HUD Ref`) "«Осколки. Я разбила его сама? Или... оно разбилось, потому что я не могла смотреть на себя?» \n«Нужно найти 4 осколка. Нужно собрать их и узнать всю правду.» \n"))))

(fn `GetItemType`
  (returns (Type :type Integer))
  (return 1))

(fn `UserConstructionScript`
  (`parent.UserConstructionScript`))