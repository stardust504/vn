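; BP_MirrorNormal is an interactable mirror that shows the player character's self-admiring Russian monologue line when used.
; One second after BeginPlay it casts the player character to BP_MyCharacter and caches it along with its HUD reference.
; Interact checks that the HUD is valid, clears its text and prints the hardcoded line.
; GetItemType reports a fixed type of 1.
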(event `self.ReceiveBeginPlay`
  (`parent.ReceiveBeginPlay`)
  (`KismetSystemLibrary.Delay` 1.0)
  (bind _asbp_my_character (cast `/Game/PlayerSystem/BP_MyCharacter` (`GameplayStatics.GetPlayerCharacter` 0)))
  (bind _output_get (set `self.Character` _asbp_my_character))
  (set `self.HUD` (`/Game/PlayerSystem/BP_MyCharacter.HUD_Ref` _output_get)))

(event `/Game/Interactables/BPI_Interact.Interact`
  (bind _hud (`self.HUD`))
  (`/Engine/EditorBlueprintResources/StandardMacros.IsValid` _hud
    (:`Is Valid`
      (`/Game/UI/Widgets/WBP_HUD.ClearText` _hud)
      (`/Game/UI/Widgets/WBP_HUD.PrintText` _hud "«Какая я сегодня красивая... Нет. Не сегодня. Я всегда такая. Просто раньше не замечала.»"))))

(fn `GetItemType`
  (returns (Type :type Integer))
  (return 1))

(fn `UserConstructionScript`
  (`parent.UserConstructionScript`))