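; BP_Collectible_Shard is an interactable memory shard pickup that reports a fixed item type.
; On Interact it plays a pickup sound at a hardcoded world location, then has BP_MyCharacter start its shard collection animation with the mesh, memory image, text and shard ID.
; The actor then destroys itself, provided the player character cast succeeded.
; The construction script applies ItemMesh to the static mesh component.
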(event `/Game/Interactables/BPI_Interact.Interact`
  (`GameplayStatics.PlaySoundAtLocation` "/Game/Audio/SFX/A_Shard_Pickup.A_Shard_Pickup" (10.0 0.0 0.0) (struct) 1.0 1.0 0.0 null null null null)
  (bind _asbp_my_character (cast `/Game/PlayerSystem/BP_MyCharacter` (`GameplayStatics.GetPlayerCharacter` 0)))
  (`/Game/PlayerSystem/BP_MyCharacter.StartCollectShardAnimation` _asbp_my_character (`self.Item_Mesh`) (`self.Item_Image`) (`self.Item_Text`) (`self.Shard_ID`))
  (`self.K2_DestroyActor`))

(fn `GetItemType`
  (returns (Type :type Integer))
  (return 2))

(fn `UserConstructionScript`
  (`StaticMeshComponent.SetStaticMesh` (`self.StaticMesh`) (`self.Item_Mesh`))
  (`parent.UserConstructionScript`))