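; BP_Phone is an interactable phone that launches a phone minigame when the player interacts with it.
; On BeginPlay it casts player controller 0 to BP_MyPlayerController and caches the reference.
; Its Interact event checks that reference is valid, then calls StartMiniGame on the controller with the WBP_Minigame_Phone widget.
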(event `self.ReceiveBeginPlay`
  (`parent.ReceiveBeginPlay`)
  (bind _asbp_my_player_controller (cast `/Game/PlayerSystem/BP_MyPlayerController` (`GameplayStatics.GetPlayerController` 0)))
  (set `self.MyPlayerController` _asbp_my_player_controller))

(event `/Game/Interactables/BPI_Interact.Interact`
  (bind _myplayercontroller (`self.MyPlayerController`))
  (`/Engine/EditorBlueprintResources/StandardMacros.IsValid` _myplayercontroller
    (:`Is Valid`
      (`/Game/PlayerSystem/BP_MyPlayerController.StartMiniGame` _myplayercontroller "/Game/UI/Widgets/WBP_Minigame_Phone.WBP_Minigame_Phone_C"))))

(fn `UserConstructionScript`
  (`parent.UserConstructionScript`))