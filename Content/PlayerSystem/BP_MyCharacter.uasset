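; First-person player character that handles movement, look, interaction and memory shard collection.
; A short camera trace each tick sets the HUD cursor from BPI_Interact item types, while IA_Interact repeats the trace to message the hit actor.
; A timeline with interpolation bobs the camera while moving.
; Collecting a shard increments the count, disables input, starts the HUD memory sequence and animates an inspect mesh via timeline.
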(event `self.ReceiveTick`
  (params (DeltaSeconds :type "Float (single-precision)"))
  (bind _returnvalue (`SceneComponent.K2_GetComponentLocation` (`self.Camera`)))
  (`|ExecutionSequence`
    (:`then_0`
      ;[1 1 1] Изменение курсора
      (bind _outhit (`KismetSystemLibrary.LineTraceSingle` _returnvalue (+ _returnvalue (* (`SceneComponent.GetForwardVector` (`self.Camera`)) 200.0)) "TraceTypeQuery1"))
      (bind (_bblockinghit _binitialoverlap _time _distance _location _impactpoint _normal _impactnormal _physmat _hitactor) (`GameplayStatics.BreakHitResult` _outhit))
      (if _bblockinghit
        (if (`KismetSystemLibrary.DoesImplementInterface` _hitactor "/Game/Interactables/BPI_Interact.BPI_Interact_C")
          (bind _type (message `/Game/Interactables/BPI_Interact.GetItemType` _hitactor))
          (`/Game/UI/Widgets/WBP_HUD.UpdateCursor` (`self.HUD_Ref`) _type)
          (else
            (`/Game/UI/Widgets/WBP_HUD.UpdateCursor` (`self.HUD_Ref`) 0)))
        (else
          (`/Game/UI/Widgets/WBP_HUD.UpdateCursor` (`self.HUD_Ref`) 0))))
    (:`then_1`
      ;[1 1 1] Покачивание камеры
      (if (> (`KismetMathLibrary.VSize` (`self.GetVelocity`)) 0.0)
        ;;[0.5806 0.8254 1] Анимация покачивания
        (bind (_direction _bob) (`Timeline|Timeline` :!label _label)
          (:`Update`
            (`SceneComponent.K2_SetRelativeLocation` (`self.Camera`) (`KismetMathLibrary.MakeVector` 0.0 0.0 (`KismetMathLibrary.FInterpTo` (.z (`SceneComponent.RelativeLocation` (`self.Camera`))) (* _bob (`self.BobAmount`)) (`GameplayStatics.GetWorldDeltaSeconds`) 6.0)) false false)))
        (else
          (`SceneComponent.K2_SetRelativeLocation` (`self.Camera`) (`KismetMathLibrary.MakeVector` 0.0 0.0 (`KismetMathLibrary.FInterpTo` (.z (`SceneComponent.RelativeLocation` (`self.Camera`))) 0.0 DeltaSeconds 5.0)) false false)
          (goto _label :!via `Stop`))))))

(event `StartCollectShardAnimation`
  (params (MeshToInspect :type "StaticMesh Object Reference") (MemoryImage :type "Texture2D Object Reference") (MemoryText :type "Array of Text") (Shard_ID :type Integer))
  (bind _inspect_mesh (`self.Inspect_Mesh`))
  (bind _inspect_mesh_2 (`self.Inspect_Mesh`))
  ;[1 1 1] Нужно для подсчета сколько собрано: делает +1 за каждый осколок
  (set `self.CollectedShards` (+ (`self.CollectedShards`) 1))
  (`/Game/UI/Widgets/WBP_HUD.AddShardIcon` (`self.HUD_Ref`) Shard_ID)
  (`self.DisableInput` (`GameplayStatics.GetPlayerController` 0))
  (`WidgetBlueprintLibrary.SetInputMode_UIOnlyEx` (`GameplayStatics.GetPlayerController` 0) (`self.HUD_Ref`))
  (`/Game/UI/Widgets/WBP_HUD.StartMemorySequence` (`self.HUD_Ref`) MemoryImage MemoryText)
  (`StaticMeshComponent.SetStaticMesh` _inspect_mesh MeshToInspect)
  (`SceneComponent.SetVisibility` _inspect_mesh true false)
  (bind (_direction _location _rotation) (`Timeline|CollectShardAnimationTimeLine` :!via `PlayFromStart`)
    (:`Update`
      (`|ExecutionSequence`
        (:`then_0`
          (`SceneComponent.K2_SetRelativeLocation` _inspect_mesh_2 _location false false))
        (:`then_1`
          (`SceneComponent.K2_SetRelativeRotation` _inspect_mesh_2 (`KismetMathLibrary.MakeRotator` (.x _rotation) (.y _rotation) (.z _rotation)) false false))))
    (:`Finished`
      (`SceneComponent.SetVisibility` (`self.Inspect_Mesh`) false false))))

(event `self.ReceiveBeginPlay`
  (`/Engine/EditorBlueprintResources/StandardMacros.IsValid` (`self.HUD_Ref`)
    (:`Is Not Valid`
      ;[0.7476 0.9083 1] Вывод интерфейса
      (bind _returnvalue (`|CreateWidget` "/Game/UI/Widgets/WBP_HUD.WBP_HUD_C"))
      (bind _output_get (set `self.HUD_Ref` _returnvalue))
      (`UserWidget.AddToViewport` _output_get 0)
      (bind _asplayer_controller (cast `PlayerController` (`self.GetController`)))
      (`EnhancedInputSubsystemInterface.AddMappingContext` (pcsubsystem `EnhancedInputLocalPlayerSubsystem` _asplayer_controller) "/Game/PlayerSystem/IMC_Default.IMC_Default" 0 (struct))
      (`KismetSystemLibrary.PrintString` "Hello"))))

(event `EnhancedInput|/Game/PlayerSystem/IA_Move`
  (params (ActionValue :type "Vector2D Structure") (ElapsedSeconds :type "Float (double-precision)") (TriggeredSeconds :type "Float (double-precision)") (InputAction :type "InputAction Object Reference" :default "/Game/PlayerSystem/IA_Move.IA_Move"))
  (bind (_x _y) (`KismetMathLibrary.BreakVector2D` ActionValue))
  ;[1 1 1] Оси движение по WASD, Вращение мышью (IA_Move, IA_Look)
  (:`Triggered`
    (`self.AddMovementInput` (`self.GetActorForwardVector`) _x)
    (`self.AddMovementInput` (`self.GetActorRightVector`) _y)))

(event `EnhancedInput|/Game/PlayerSystem/IA_Look`
  (params (ActionValue :type "Vector2D Structure") (ElapsedSeconds :type "Float (double-precision)") (TriggeredSeconds :type "Float (double-precision)") (InputAction :type "InputAction Object Reference" :default "/Game/PlayerSystem/IA_Look.IA_Look"))
  (bind (_x _y) (`KismetMathLibrary.BreakVector2D` ActionValue))
  ;[1 1 1] Оси движение по WASD, Вращение мышью (IA_Move, IA_Look)
  (:`Triggered`
    (`self.AddControllerYawInput` _x)
    (`self.AddControllerPitchInput` _y)))

(event `Key|LeftMouseButton`
  (params (Key :type "Key Structure"))
  ;[1 1 1] ЛКМ
)

(event `EnhancedInput|/Game/PlayerSystem/IA_Interact`
  (params (ActionValue :type Boolean) (ElapsedSeconds :type "Float (double-precision)") (TriggeredSeconds :type "Float (double-precision)") (InputAction :type "InputAction Object Reference" :default "/Game/PlayerSystem/IA_Interact.IA_Interact"))
  (bind _returnvalue (`SceneComponent.K2_GetComponentLocation` (`self.Camera`)))
  ;[1 1 1] ЛКМ
  (:`Started`
    (bind _outhit (`KismetSystemLibrary.LineTraceSingle` :`Start` _returnvalue :`End` (+ _returnvalue (* (`SceneComponent.GetForwardVector` (`self.Camera`)) 200.0)) :`TraceChannel` "TraceTypeQuery1" :`DrawDebugType` "Persistent"))
    (message `/Game/Interactables/BPI_Interact.Interact` (`.HitActor` (`GameplayStatics.BreakHitResult` _outhit)))))

(fn `UserConstructionScript`)