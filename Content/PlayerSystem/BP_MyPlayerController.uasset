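; Player controller that handles switching to interactable cameras and running widget-based minigames.
; SwitchTargetCameraToInteract blends the view to a stored camera, disables input and shows the cursor.
; StartMiniGame opens a given widget in UI-only mode and, for the phone minigame, binds its exit request to CloseWidget.
; CloseWidget restores game input and, after a short delay, sends an open-door message to actors tagged "door2".
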(event `SwitchTargetCameraToInteract`
  (`self.SetViewTargetWithBlend` (`self.InteractableCamera`))
  (`self.DisableInput` self)
  (`WidgetBlueprintLibrary.SetInputMode_GameAndUIEx` self null)
  (set `self.bShowMouseCursor` true))

(event `StartMiniGame`
  (params (MinigameClass :type "UserWidget Class Reference"))
  (bind _returnvalue (`|CreateWidget` MinigameClass))
  (bind _output_get (set `self.MinigameWidget` _returnvalue))
  (`UserWidget.AddToViewport` _output_get 0)
  (`WidgetBlueprintLibrary.SetInputMode_UIOnlyEx` self null)
  (set `self.bShowMouseCursor` true)
  (bind _aswbp_minigame_phone (cast `/Game/UI/Widgets/WBP_Minigame_Phone` (`self.MinigameWidget`)))
  (add `/Game/UI/Widgets/WBP_Minigame_Phone.OnRequestExit` _aswbp_minigame_phone (delegate `CloseWidget`)))

(event `CloseWidget`
  (`Widget.RemoveFromParent` (`self.MinigameWidget`))
  (`WidgetBlueprintLibrary.SetInputMode_GameOnly` self)
  (set `self.bShowMouseCursor` false)
  (`KismetSystemLibrary.Delay` 1.0)
  (bind _outactors (`GameplayStatics.GetAllActorsWithTag` "door2"))
  (for _array_element _outactors
    (message `/Game/Assets/Door/BPI_Door.OpenDoor` _array_element)))

(fn `SetInteractableCamera`
  (params (InteractableClass :type "Actor Object Reference"))
  (set `self.InteractableCamera` InteractableClass))

(fn `UserConstructionScript`)